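; BP_Platform is a gimmick actor that moves a platform along the direction of its Arrow component.
; On BeginPlay it waits a random fraction of a second, likely to desynchronize instances, then stores its origin and plays the Move timeline.
; Each timeline update sets the location to the origin plus the arrow's forward vector scaled by MoveLength and Alpha, without sweeping.
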(event `self.ReceiveBeginPlay`
  (`KismetSystemLibrary.Delay` (`KismetMathLibrary.RandomFloat`))
  (set `self.OriginLocation` (`self.K2_GetActorLocation`))
  (bind (_direction _alpha) (`Timeline|Move`)
    (:`Update`
      (`self.K2_SetActorLocation` (+ (`self.OriginLocation`) (* (`SceneComponent.GetForwardVector` (`self.Arrow`)) (`self.MoveLength`) _alpha))))))

(fn `UserConstructionScript`)