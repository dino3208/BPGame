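; BP_LevelLoadTrigger is a gimmick actor that streams in its TargetLevel when an actor tagged Player overlaps it.
; It performs a blocking load with visibility off, prints a Korean "loaded" debug message, then looks up the streaming level by object name and sets it visible.
; A 3-second Delay leading to the visibility step is disconnected and never runs.
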(event `self.ReceiveActorBeginOverlap`
  (params (OtherActor :type "Actor Object Reference"))
  (if (`self.ActorHasTag` OtherActor "Player")
    (`GameplayStatics.LoadStreamLevelBySoftObjectPtr` (`self.TargetLevel`) false true)
    (`KismetSystemLibrary.PrintString` "로드됨")
    (set `LevelStreaming.bShouldBeVisible` true (`GameplayStatics.GetStreamingLevel` (`KismetStringLibrary.Conv_StringToName` (`KismetSystemLibrary.GetObjectName` (`|ConvertAsset` (`self.TargetLevel`))))))))

(fn `UserConstructionScript`)