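; Bear monster character with sight-driven chasing, damage feedback and death handling.
; A state setter writes the state to the AI blackboard and sets walk speed from monster stats, ignoring changes once dead.
; Seeing a Player-tagged pawn during locomotion sets it on the blackboard and starts the chase.
; Damage feeds the stat component and a timeline-driven material flash; zero HP disables collision, stops AI, plays a death montage, then destroys the actor.
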(event `self.ReceiveBeginPlay`
  ; 머터리얼 인스턴스 생성 (피격효과)
  (bind _returnvalue (`PrimitiveComponent.CreateDynamicMaterialInstance` (`self.Mesh`) 0 "/Game/InfinityBladeAdversaries/Enemy/Enemy_Bear/Materials/M_Bear_Stone_Inst.M_Bear_Stone_Inst" "None"))
  (set `self.MaterialInstance` _returnvalue)
  ; 죽음 이벤트 등록 및 처리
  (add `/Game/Blueprints/Game/Component/BP_MonsterStat.OnHpZero` (`self.BP_MonsterStat`) (delegate `MonsterDied`)))

(event `MonsterDied`
  (bind _braincomponent (`AIController.BrainComponent` (`AIBlueprintHelperLibrary.GetAIController` self)))
  ; 죽음 이벤트 등록 및 처리
  (`self.SetActorEnableCollision` false) ; 액터의 모든 콜리전 끄기
  (`self.PlayAnimMontage` "/Game/Blueprints/Game/Monster/Animation/AM_MonsterDead.AM_MonsterDead")
  ;;[0 0 0 0.5] AI 중지 처리
  (`BrainComponent.StopLogic` _braincomponent "")
  (message `NavMovementInterface.StopActiveMovement` _braincomponent)
  (`self.SetState` "NewEnumerator3")
  (`KismetSystemLibrary.Delay` 2.0)
  (`self.K2_DestroyActor`))

(event `self.ReceiveAnyDamage`
  (params (Damage :type "Float (single-precision)") (DamageType :type "DamageType Object Reference") (InstigatedBy :type "Controller Object Reference") (DamageCauser :type "Actor Object Reference"))
  ; 몬스터 데미지 처리
  (`self.PlayDamageEffect`)
  (`/Game/Blueprints/Game/Component/BP_MonsterStat.ReceiveDamage` (`self.BP_MonsterStat`) Damage))

(event `PlayDamageEffect`
  ; 피격 효과
  (bind (_direction _alpha) (`Timeline|DamageEffect` :!via `PlayFromStart`)
    (:`Update`
      (bind _materialinstance (`self.MaterialInstance`)
        (:`then`
          (`MaterialInstanceDynamic.SetScalarParameterValue` _materialinstance "DamageFactor" _alpha))
        (:`else`)))
    (:`Finished`
      (bind _materialinstance_2 (`self.MaterialInstance`)
        (:`then`
          (`MaterialInstanceDynamic.SetScalarParameterValue` _materialinstance_2 "DamageFactor" 0.0))
        (:`else`)))))

(event `self.PawnSensing.OnSeePawn`
  (params (Pawn :type "Pawn Object Reference"))
  (switch `/Game/Blueprints/Game/Monster/EBearState` (`self.BearState`)
    (:`NewEnumerator0`
      (if (`self.ActorHasTag` Pawn "Player")
        (`BlackboardComponent.SetValueAsObject` (`AIBlueprintHelperLibrary.GetBlackboard` (`AIBlueprintHelperLibrary.GetAIController` self)) (`self.Key Name`) Pawn)
        (`self.SetState` "NewEnumerator1")))))

(fn `SetState`
  (params (NewState :type "/Game/Blueprints/Game/Monster/EBearState Enum" :default "NewEnumerator0"))
  (bind _charactermovement (`self.CharacterMovement`))
  (bind (_monsterstat_maxhp _monsterstat_walkspeed _monsterstat_chasespeed) (break `/Game/Blueprints/Game/Monster/Data/FMonsterData` (`/Game/Blueprints/Game/Monster/Data/BP_MonsterData.MonsterStat` (`/Game/Blueprints/Game/Component/BP_MonsterStat.MonsterData` (`self.BP_MonsterStat`)))))
  (if (`|EnumInequality` (`self.BearState`) "NewEnumerator3")
    (bind _output_get (set `self.BearState` NewState))
    (`BlackboardComponent.SetValueAsEnum` (`AIController.Blackboard` (`AIBlueprintHelperLibrary.GetAIController` self)) (`self.StateKey`) _output_get)
    (switch `/Game/Blueprints/Game/Monster/EBearState` (`self.BearState`)
      (:`NewEnumerator0`
        (set `CharacterMovementComponent.MaxWalkSpeed` _monsterstat_walkspeed _charactermovement))
      (:`NewEnumerator1`
        (set `CharacterMovementComponent.MaxWalkSpeed` _monsterstat_chasespeed _charactermovement))
      (:`NewEnumerator2`
        (set `CharacterMovementComponent.MaxWalkSpeed` 0.0 _charactermovement :!label _label))
      (:`NewEnumerator3`
        (goto _label)))))

(fn `UserConstructionScript`)